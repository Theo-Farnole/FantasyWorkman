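; BP_CharaTest is a test character that moves along world X and Y and triggers pickup of BP_PickUpObjectByTwo objects.
; The WhichControl flag selects which of two input axis sets drives movement: UpDown/LeftRight when true, HautBas/GaucheDroite when false.
; When its capsule hits a BP_PickUpObjectByTwo, it registers itself as that object's Chara1 and sets its PickUp flag.
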(event OnComponentHit(CapsuleComponent)
  (params (HitComponent :type Primitive%20Component%20Object%20Reference) (OtherActor :type Actor%20Object%20Reference) (OtherComp :type Primitive%20Component%20Object%20Reference) (NormalImpulse :type Vector :default "0, 0, 0") (Hit :type Hit%20Result%20Structure%20%28by%20ref%29))
  (if (== (Utilities|GetClass OtherActor) "/Game/Blueprints/Technical/Test/Trash/BP_PickUpObjectByTwo.BP_PickUpObjectByTwo_C")
    (bind _asbp_pick_up_object_by_two (Utilities|Casting|CastToBP_PickUpObjectByTwo OtherActor))
    (Variables|/Game/Blueprints/Technical/Test/Trash/BP_PickUpObjectByTwo.BP_PickUpObjectByTwo_C|Setchara1 _asbp_pick_up_object_by_two self)
    (Variables|/Game/Blueprints/Technical/Test/Trash/BP_PickUpObjectByTwo.BP_PickUpObjectByTwo_C|SetPickUp _asbp_pick_up_object_by_two true)))

(event EventBeginPlay)

(event Collision|EventActorBeginOverlap
  (params (OtherActor :type Actor%20Object%20Reference)))

(event EventTick
  (params (DeltaSeconds :type Float%20%28single-precision%29)))

(event Input|AxisEvents|InputAxisUpDown
  (params (AxisValue :type Float%20%28single-precision%29))
  (if (Variables|Default|GetwhichControl)
    (Pawn|Input|AddMovementInput "1.000000, 0, 0" (stale Input|AxisEvents|InputAxisHautBas AxisValue) false)))

(event Input|AxisEvents|InputAxisLeftRight
  (params (AxisValue :type Float%20%28single-precision%29))
  (if (Variables|Default|GetwhichControl)
    (Pawn|Input|AddMovementInput "0,1.000000, 0" (stale Input|AxisEvents|InputAxisGaucheDroite AxisValue) false)))

(event Input|AxisEvents|InputAxisHautBas
  (params (AxisValue :type Float%20%28single-precision%29))
  (if (not (Variables|Default|GetwhichControl))
    (Pawn|Input|AddMovementInput "1.000000, 0, 0" AxisValue false)))

(event Input|AxisEvents|InputAxisGaucheDroite
  (params (AxisValue :type Float%20%28single-precision%29))
  (if (not (Variables|Default|GetwhichControl))
    (Pawn|Input|AddMovementInput "0,1.000000, 0" AxisValue false)))

(fn ConstructionScript)