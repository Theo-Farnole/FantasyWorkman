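; Actor component that shows or hides a colored outline around its owner using a configurable static mesh, optionally at BeginPlay.
; Because it cannot add a mesh component, it spawns a StaticMeshActor attached to the owner, ignoring one custom trace channel.
; That mesh gets a dynamic M_Outline material on slot 0, driven by color and scale.
; Hiding destroys the spawned actor, whose validity also reports whether the outline is shown.
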(event EventTick
  (params (DeltaSeconds :type Float%20%28single-precision%29)))

(event EventBeginPlay
  (if (Variables|Default|GetoutlineAtStart)
    (CallFunction|ShowOutline)))

(fn ShowOutline
  (CallFunction|HideOutline)
  (bind _outline (Utilities|AddStaticMeshComponent))
  (Components|StaticMesh|SetStaticMesh (Variables|/Script/Engine.StaticMeshActor|GetStaticMeshComponent _outline) (Variables|Mesh|GetStaticMesh))
  (Utilities|ApplyOutlineMaterialonStaticMesh (Variables|/Script/Engine.StaticMeshActor|GetStaticMeshComponent _outline))
  (return))

(fn HideOutline
  (Utilities|IsValid (Variables|Default|Getoutline)
    (:Is%20Valid
      (Actor|DestroyActor (Variables|Default|Getoutline)))))

(fn IsOutlineShow
  (return (Utilities|IsValid (Variables|Default|Getoutline))))