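; Scene component that lets its owner carry, drop and throw one object at a time.
; Carry attaches the object to the component at a grab location and disables its physics and collision.
; Uncarry restores both, detaches it and clears the reference, notifying the object as Carry does.
; Throwing requires BP_IThrowable approval, then uncarries, applies a velocity-change impulse and calls OnThrow, with invalid calls printing errors.
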(fn Carry
  (params (object :type BP%20I%20Carriable%20Interface) (grabLocation :type Vector))
  ;[1 1 1] Do object to carry is valid ?
  (Utilities|IsValid (Utilities|ToObject(Interface) object)
    (:Is%20Valid
      ;[1 1 1] Prevent carry if the player already carry something
      (Utilities|IsValid (Utilities|ToObject(Interface) (Variables|Default|GetcarriedObject))
        (:Is%20Valid
          (Development|PrintString "ERROR: cannot call Carry while Carrier is already carrying an object."))
        (:Is%20Not%20Valid
          (bind _output_get (Variables|Default|SetcarriedObject object))
          (Utilities|AttachCarriedObjecttoAnchor _output_get grabLocation)
          (Default|OnCarry _output_get self))))
    (:Is%20Not%20Valid
      (Development|PrintString "ERROR: cannot call Carry if the parameter \"Object\" is not valid."))))

(fn Uncarry
  (bind _detachactorrule (LocalVariables|GetdetachActorRule))
  ;[1 1 1] Prevent uncarry if the carrier doesn't carry anything
  (Utilities|IsValid (Utilities|ToObject(Interface) (Variables|Default|GetcarriedObject))
    (:Is%20Valid
      (Utilities|FlowControl|Sequence
        (:then_0
          ;[1 1 1] Reactive physics
          (bind _cariablecomponent (Default|GetCariableComponent (Variables|Default|GetcarriedObject)))
          (Utilities|ActivePhysicsandCollision _cariablecomponent))
        (:then_1
          ;[1 1 1] Deattach
          (bind _asactor (Utilities|Casting|CastToActor (Utilities|ToObject(Interface) (Variables|Default|GetcarriedObject))))
          (Transformation|DetachFromActor _asactor _detachactorrule _detachactorrule _detachactorrule))
        (:then_2
          ;[1 1 1] Call OnUncarry and remove reference to carried object.
          (Default|OnUncarry (Variables|Default|GetcarriedObject) self)
          (Variables|Default|SetcarriedObject 0))))
    (:Is%20Not%20Valid
      (Development|PrintString "ERROR: Cannot uncarry if the Carrier doesn't carry anything."))))

(fn ThrowCarriedObject
  (bind _returnvalue (Utilities|GetThrowForceVector))
  (bind _carriedobject (Variables|Default|GetcarriedObject))
  (Utilities|IsValid (Utilities|ToObject(Interface) (Variables|Default|GetcarriedObject))
    (:Is%20Valid
      (bind _ithrowable (Utilities|CanbeThrow)
        (:Throwable
          (bind _cariablecomponent (Default|GetCariableComponent _carriedobject))
          (Utilities|IsValid _cariablecomponent
            (:Is%20Valid
              (CallFunction|Uncarry)
              (Utilities|ActivePhysicsandCollision _cariablecomponent)
              (Physics|AddImpulse _cariablecomponent _returnvalue "None" true)
              (Default|OnThrow _ithrowable (Components|GetOwner) _returnvalue)
              (return))
            (:Is%20Not%20Valid
              (Development|PrintString (Utilities|String|Append "ERROR: GetCarriable returns null." (Utilities|GetDisplayName (Utilities|ToObject(Interface) _carriedobject)))))))
        (:NotThrowable
          (Development|PrintString "ERROR: This item can't be throw."))))
    (:Is%20Not%20Valid
      (Development|PrintString "ERROR: Cannot throw if the carrier doesn't carry an item."))))

(fn CanThrowCarriedObject
  (bind (_asbp_ithrowable _succesful) (CallFunction|GetIThrowable true))
  (if _succesful
    (bind _throwable (Default|CanThrow _asbp_ithrowable))
    (return _throwable)
    (else
      (return false))))

(fn GetIThrowable
  (params (logErrors :type Boolean))
  (Utilities|IsValid (Utilities|ToObject(Interface) (Variables|Default|GetcarriedObject))
    (:Is%20Valid
      (bind _asbp_ithrowable (Utilities|Casting|CastToBP_IThrowable (Variables|Default|GetcarriedObject))
        (:then
          (return _asbp_ithrowable true))
        (:CastFailed
          (if logErrors
            (Development|PrintString "ERROR: Cannot throw an item that doesn't have implemented interface Thowable")
            (return 0 false)))))
    (:Is%20Not%20Valid
      (if logErrors
        (Development|PrintString "ERROR: Carrier cannot Throw() if it doesn't carry anything.")
        (return 0 false)))))