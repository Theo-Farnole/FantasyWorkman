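; Character component that tracks the nearest hoverable object and shows its interaction prompt for the third-person character.
; Each tick it queries the character's detection component, and only when the target changes sends EndHover and StartHover and updates the UI widget component.
; A cast chain picks the prompt: items, piles and ChopChop workshops get an interaction widget that reflects what is carried, while pulley actioners get a simple icon.
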(event EventBeginPlay
  (CallFunction|SetVariablesCharacter))

(event EventTick
  (params (DeltaSeconds :type Float%20%28single-precision%29))
  (bind (_hoverablefound _hoverable) (Default|GetNearestHoverable (Variables|Default|GetCharacterDetection)))
  (if _hoverablefound
    _
    (else
      _))
  (Utilities|SetHoverable _hoverable))

(fn SetVariablesCharacter
  (bind _asch_third_person (Utilities|Casting|CastToCH_ThirdPerson (Components|GetOwner)))
  (bind _output_get (Variables|Default|SetCharacter _asch_third_person))
  (Variables|Default|SetCharacterDetection (Variables|/Game/Blueprints/Gamemodes/Game/CH_ThirdPerson.CH_ThirdPerson_C|GetBPC_CharacterDetection _output_get))
  (Variables|Default|SetWidgetUpdate (Variables|/Game/Blueprints/Gamemodes/Game/CH_ThirdPerson.CH_ThirdPerson_C|GetBPC_UIWidgeUpdate _asch_third_person)))

(fn HideSprite
  (params (Chara :type CH%20Third%20Person%20Object%20Reference))
  (Default|HideWidget (Variables|/Game/Blueprints/Gamemodes/Game/CH_ThirdPerson.CH_ThirdPerson_C|GetBPC_UIWidgeUpdate Chara)))