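; Component for a BP_AConstructionToBuild owner (the bridge) that shows an overhead icon widget with a count of contents needed.
; On BeginPlay it caches the owner, and each Tick it projects that actor's location to screen space to position the widget, centered with a fixed offset.
; Functions create the WPB_IconOverHead widget if none is valid, update its needed count, or remove it from its parent.
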(event EventBeginPlay
  (Utilities|GetBridge))

(event EventTick
  (params (DeltaSeconds :type Float%20%28single-precision%29))
  (bind _currentswidget (Variables|Default|GetCurrentsWidget))
  (Utilities|IsValid _currentswidget
    (:Is%20Valid
      (Class|UserWidget|SetPositioninViewport _currentswidget (+ (- (.ScreenPosition (Class|WidgetLayoutLibrary|ProjectWorldLocationtoWidgetPosition (Game|GetPlayerController 0) (Transformation|GetActorLocation (Variables|Default|GetBridge)) false)) (* (Class|Widget|GetDesiredSize (Variables|Default|GetCurrentsWidget)) 0.5)) "(X=50.000000,Y=-90.000000)") false))))

(fn ShowNumberedIcon
  (params (Icon :type Texture%202D%20Object%20Reference) (contentsNeeded :type Integer))
  (Utilities|IsValid (Variables|Default|GetCurrentsWidget)
    (:Is%20Not%20Valid
      (CallFunction|HideWidget)
      (bind _returnvalue (UserInterface|CreateWidget "/Game/Blueprints/Widgets/WPB_IconOverHead.WPB_IconOverHead_C"))
      (bind _output_get (Variables|Default|SetCurrentsWidget _returnvalue))
      (Default|SetIconBridge _output_get Icon)
      (Variables|/Game/Blueprints/Widgets/WPB_IconOverHead.WPB_IconOverHead_C|SetcontentNeeds _returnvalue contentsNeeded)
      (UserInterface|Viewport|AddtoPlayerScreen _returnvalue -2))))

(fn HideWidget
  (bind _currentswidget (Variables|Default|GetCurrentsWidget))
  (Utilities|IsValid _currentswidget
    (:Is%20Valid
      (Widget|RemovefromParent _currentswidget))))

(fn UpdateWidget
  (params (ContentsNeed :type Integer))
  (Variables|/Game/Blueprints/Widgets/WPB_IconOverHead.WPB_IconOverHead_C|SetcontentNeeds (Variables|Default|GetCurrentsWidget) ContentsNeed))