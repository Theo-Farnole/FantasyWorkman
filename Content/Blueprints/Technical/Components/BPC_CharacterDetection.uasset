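; Character detection component that finds hoverable, interactable and carriable actors in front of its owner.
; A shared forward capsule trace on one trace channel feeds three getters, each casting the hit actor to its matching interface.
; BeginPlay caches the owner as CH_ThirdPerson.
; Tick runs the hoverable query every frame but does not use its result here.
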(event EventBeginPlay
  (CallFunction|GetCharacter))

(event EventTick
  (params (DeltaSeconds :type Float%20%28single-precision%29))
  (CallFunction|GetNearestHoverable))

(fn GetNearestHoverable
  (bind (_outhit _return) (Utilities|CapsuleTrace))
  (if _return
    (bind _asbp_ihoverable (Utilities|Casting|CastToBP_IHoverable (.HitActor (Collision|BreakHitResult _outhit)))
      (:then
        (return true _asbp_ihoverable))
      (:CastFailed
        (return false 0)))
    (else
      (return false 0))))

(fn GetNearestInteractable
  (bind (_outhit _return) (Utilities|CapsuleTrace))
  (if _return
    (bind _asbp_iinteractable (Utilities|Casting|CastToBP_IInteractable (.HitActor (Collision|BreakHitResult _outhit)))
      (:then
        (return true _asbp_iinteractable))
      (:CastFailed
        (return false 0)))
    (else
      (return false 0))))

(fn GetNearestCarriable
  (bind (_outhit _return) (Utilities|CapsuleTrace))
  (if _return
    (bind _asbp_icarriable (Utilities|Casting|CastToBP_ICarriable (.HitActor (Collision|BreakHitResult _outhit)))
      (:then
        (return true _asbp_icarriable))
      (:CastFailed
        (return false 0)))
    (else
      (return false 0))))

(fn GetCharacter
  (bind _asch_third_person (Utilities|Casting|CastToCH_ThirdPerson (Components|GetOwner)))
  (Variables|Default|SetCharacter _asch_third_person))