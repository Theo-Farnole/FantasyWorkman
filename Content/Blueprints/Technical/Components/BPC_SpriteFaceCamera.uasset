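; Actor component meant to billboard the IconUI sprite of a CH_ThirdPerson owner toward the player camera.
; BeginPlay casts the owner and caches its sprite; Tick sets that sprite's relative rotation from FaceCamera while it is valid.
; FaceCamera holds an offset look-at rotation from camera to sprite, but that calculation is unused, with no return shown.
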(event EventBeginPlay
  (CallFunction|GetCharacter))

(event EventTick
  (params (DeltaSeconds :type Float%20%28single-precision%29))
  (Utilities|IsValid (Variables|Default|Getsprite)
    (:Is%20Valid
      (Transformation|SetRelativeRotation (Variables|Default|Getsprite) (Utilities|FaceCamera) false false))))

(fn GetCharacter
  (bind _asch_third_person (Utilities|Casting|CastToCH_ThirdPerson (Components|GetOwner)))
  (bind _output_get (Variables|Default|SetCharacter _asch_third_person))
  (Variables|Default|Setsprite (Variables|/Game/Blueprints/Gamemodes/Game/CH_ThirdPerson.CH_ThirdPerson_C|GetIconUI _output_get)))