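; Actor component for CH_ThirdPerson that shows icon prompt widgets on screen at the character's position.
; Show functions create an interaction widget, with a needed-item or input circle icon, or a simple icon widget, and store it as CurrentWidget for HideWidget to remove.
; Each tick it projects the character's world location to screen space to reposition that widget.
; ShowNumberedIconWidget is an empty stub, and FaceCamera holds only unused rotation math.
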(event EventBeginPlay
  (CallFunction|GetCharacter))

(event EventTick
  (params (DeltaSeconds :type Float%20%28single-precision%29))
  (Utilities|WidgetFollowPlayer))

(fn GetCharacter
  (bind _asch_third_person (Utilities|Casting|CastToCH_ThirdPerson (Components|GetOwner)))
  (bind _output_get (Variables|Default|SetCharacter _asch_third_person))
  (Variables|Default|Setsprite (Variables|/Game/Blueprints/Gamemodes/Game/CH_ThirdPerson.CH_ThirdPerson_C|GetIconUI _output_get)))

(fn ShowInteractionWidget
  (params (IconResult :type Texture%202D%20Object%20Reference) (IconNeed :type Texture%202D%20Object%20Reference) (IconInput :type Texture%202D%20Object%20Reference) (DisplayNeedItem :type Boolean))
  (bind _returnvalue (UserInterface|CreateWidget "/Game/Blueprints/Widgets/WidgetIcon/WBP_InteractionWidget.WBP_InteractionWidget_C"))
  (bind _output_get (Variables|Default|SetCurrentWidget _returnvalue))
  (Default|SetIcon _output_get IconResult)
  (if DisplayNeedItem
    (Default|SetCircleIcon _output_get IconNeed)
    (else
      (Default|SetCircleIcon _output_get IconInput)))
  (UserInterface|Viewport|AddtoViewport _returnvalue 0))

(fn ShowSimpleIconWidget
  (params (Icon :type Texture%202D%20Object%20Reference) (IconInput :type Texture%202D%20Object%20Reference))
  (bind _returnvalue (UserInterface|CreateWidget "/Game/Blueprints/Widgets/WidgetIcon/WBP_SimpleIconWidget.WBP_SimpleIconWidget_C"))
  (bind _output_get (Variables|Default|SetCurrentWidget _returnvalue))
  (Default|SetIcon _output_get Icon)
  (Default|SetCircleIcon _output_get IconInput)
  (UserInterface|Viewport|AddtoViewport _returnvalue 0))

(fn HideWidget
  (bind _currentwidget (Variables|Default|GetCurrentWidget))
  (Utilities|IsValid _currentwidget
    (:Is%20Valid
      (Widget|RemovefromParent _currentwidget))))

(fn ShowNumberedIconWidget)