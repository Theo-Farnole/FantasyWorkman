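; BP_AItemPile is an interactable pile that hands the interacting character a newly spawned carriable item.
; Hover events toggle an outline through the static mesh outliner component.
; On interact, a CH_ThirdPerson with empty hands gets an instance of the configurable spawn class, created at the pile's transform and passed to its carrier component.
; The pile itself is never depleted; StopInteract and GetSprite are empty.
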(event EventStartInteract
  (params (interactActor :type Actor%20Object%20Reference))
  (Development|PrintString "Hello")
  (bind _asch_third_person (Utilities|Casting|CastToCH_ThirdPerson interactActor))
  (bind _holdingsomething (Default|IsCarryingSomething (Variables|/Game/Blueprints/Gamemodes/Game/CH_ThirdPerson.CH_ThirdPerson_C|GetBP_Carrier _asch_third_person)))
  (if _holdingsomething
    (Development|PrintString "Cannot pickup something while carrying.")
    (else
      (bind _returnvalue (Game|SpawnActorfromClass (Variables|Default|GetactorToSpawnOnInteract) (Transformation|GetActorTransform) "Undefined" 0 0))
      (bind _asbp_icarriable (Utilities|Casting|CastToBP_ICarriable _returnvalue)
        (:then
          (Default|Carry (Variables|/Game/Blueprints/Gamemodes/Game/CH_ThirdPerson.CH_ThirdPerson_C|GetBP_Carrier _asch_third_person) _asbp_icarriable "0, 0, 0"))
        (:CastFailed
          (Development|PrintString "ERROR: Actor to spawn cannot be carried."))))))

(event EventStopInteract
  (params (interactActor :type Actor%20Object%20Reference)))

(event EventStartHover
  (params (hoverActor :type Actor%20Object%20Reference))
  (Default|ShowOutline (Variables|Components|GetBPC_StaticMeshOutliner)))

(event EventEndHover
  (params (hoverActor :type Actor%20Object%20Reference))
  (Default|HideOutline (Variables|Components|GetBPC_StaticMeshOutliner)))

(fn ConstructionScript)

(fn GetSprite
  (return 0 0))