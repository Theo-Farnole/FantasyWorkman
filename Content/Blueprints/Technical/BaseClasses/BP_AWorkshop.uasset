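; Base actor for workshops that highlights itself through a static mesh outliner component when hovered.
; StartHover picks one of two outline states based on CanInteract for the hovering actor, and EndHover hides the outline.
; CanInteract, GetAlreadyUse and GetSprite are placeholders returning false or nothing, apparently meant for child classes to override.
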(event EventBeginPlay)

(event Collision|EventActorBeginOverlap
  (params (OtherActor :type Actor%20Object%20Reference)))

(event EventTick
  (params (DeltaSeconds :type Float%20%28single-precision%29)))

(event EventStartHover
  (params (hoverActor :type Actor%20Object%20Reference))
  (bind _isinteractable (CallFunction|CanInteract hoverActor))
  (Default|ShowOutline (Variables|Default|GetBPC_StaticMeshOutliner) (select _isinteractable "NewEnumerator1" "NewEnumerator2")))

(event EventEndHover
  (params (hoverActor :type Actor%20Object%20Reference))
  (Default|HideOutline (Variables|Default|GetBPC_StaticMeshOutliner)))

(fn ConstructionScript)

(fn GetAlreadyUse
  (return false))

(fn CanInteract
  (params (interactActor :type Actor%20Object%20Reference))
  (return false))

(fn GetSprite
  (return 0 0 0))