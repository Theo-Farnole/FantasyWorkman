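; Base actor for a buildable construction that fills up as content is added to it.
; IncrementCurrentNumbersOfContent raises the counter and calls UpdateVisual, which swaps the static mesh between unstarted and finished backfill meshes.
; Hovering toggles an outline only while the construction is unfilled, and UpdateVisual hides it once full.
; A fill-check macro drives this logic and is wrapped in an IsFill function for other classes.
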(event EventBeginPlay
  (Utilities|UpdateVisual))

(event EventStartHover
  (params (hoverActor :type Actor%20Object%20Reference))
  (if (not (Utilities|MacroIsFill))
    (Default|ShowOutline (Variables|Default|GetOutliner))))

(event EventEndHover
  (params (hoverActor :type Actor%20Object%20Reference))
  (if (not (Utilities|MacroIsFill))
    (Default|HideOutline (Variables|Default|GetOutliner))))

(fn ConstructionScript)

(fn IncrementCurrentNumbersOfContent
  (Math|Integer|IncrementInt (Variables|Default|GetcurrentNumbersOfContent)
    (:%20%20
      (Utilities|UpdateVisual))))

(fn IsFill
  ;[1 1 1] A macro is more easy to use. But we need that others classes access this.
  ; So we made a function of the macro
  (return (Utilities|MacroIsFill)))