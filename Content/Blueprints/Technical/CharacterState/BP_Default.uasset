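; BP_Default is the default character state, turning player input into movement, interaction and item handling on its owner.
; Movement follows the camera's flattened forward and right vectors, while Tick lerps the mesh toward the raw input direction at the third-person character's rotation speed.
; Interact and grab act on the nearest target from the owner's detection component.
; A carrier handles carrying, dropping and throwing.
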(event EventIStartInteract
  (bind (_isinteractable _interactable) (Default|GetNearestInteractable (Variables|/Game/Blueprints/Gamemodes/Game/CH_ThirdPerson.CH_ThirdPerson_C|GetBPC_CharacterDetection (Variables|Default|GetOwner))))
  (if _isinteractable
    (Default|StartInteract _interactable (Variables|Default|GetOwner))))

(event EventIEndInteract
  (bind (_isinteractable _interactable) (Default|GetNearestInteractable (Variables|/Game/Blueprints/Gamemodes/Game/CH_ThirdPerson.CH_ThirdPerson_C|GetBPC_CharacterDetection (Variables|Default|GetOwner))))
  (if _isinteractable
    (Default|StopInteract _interactable (Variables|Default|GetOwner))))

(event EventIUpDown
  (params (axisValue :type Float%20%28single-precision%29))
  (bind _returnvalue (Game|GetPlayerCameraManager 0))
  (bind _returnvalue_2 (Transformation|GetActorForwardVector _returnvalue))
  (bind (_x _y) (Math|Vector|BreakVector _returnvalue_2))
  (bind _output_get (Variables|Default|SetcurrentUpDown axisValue))
  (Pawn|Input|AddMovementInput (Variables|Default|GetOwner) (Math|Vector|Normalize (Math|Vector|MakeVector _x _y 0.0)) _output_get false))

(event EventILeftRight
  (params (axisValue :type Float%20%28single-precision%29))
  (bind _returnvalue (Game|GetPlayerCameraManager 0))
  (bind _returnvalue_2 (Transformation|GetActorRightVector _returnvalue))
  (bind (_x _y) (Math|Vector|BreakVector _returnvalue_2))
  (bind _output_get (Variables|Default|SetcurrentLeftRight axisValue))
  (Pawn|Input|AddMovementInput (Variables|Default|GetOwner) (Math|Vector|Normalize (Math|Vector|MakeVector _x _y 0.0)) _output_get false))

(event EventTick
  (params (DeltaSeconds :type Float%20%28single-precision%29))
  ;[1 1 1] Rotation
  (bind _returnvalue (Utilities|GetAxisValue DeltaSeconds))
  (bind _returnvalue_2 (Utilities|SetRotationbyVectorAxis _returnvalue))
  (Transformation|SetRelativeRotation (Variables|/Script/Engine.Character|GetMesh (Variables|Default|GetOwner)) _returnvalue_2 false false))

(fn SetOwner
  (params (Owner :type CH%20Third%20Person%20Object%20Reference))
  (|CallParentFunction Owner)
  (bind _asch_third_person (Utilities|Casting|CastToCH_ThirdPerson Owner))
  (Variables|Default|SetRotSpeed (Variables|/Game/Blueprints/Gamemodes/Game/CH_ThirdPerson.CH_ThirdPerson_C|GetrotationSpeed _asch_third_person)))

(fn IThrowItem
  (|CallParentFunction)
  (bind _canthrow (Default|CanThrowCarriedObject (Utilities|GetCarrier)))
  (if _canthrow
    (Default|ThrowCarriedObject (Utilities|GetCarrier))))

(fn IGrabItem
  (|CallParentFunction)
  (bind (_iscarriable _carriable) (Default|GetNearestCarriable (Variables|/Game/Blueprints/Gamemodes/Game/CH_ThirdPerson.CH_ThirdPerson_C|GetBPC_CharacterDetection (Variables|Default|GetOwner))))
  (if _iscarriable
    (Default|Carry (Utilities|GetCarrier) _carriable "0, 0, 0")))

(fn IUngrabItem
  (|CallParentFunction)
  (Default|Uncarry (Utilities|GetCarrier) true))