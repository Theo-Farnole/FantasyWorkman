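; BP_SpamInputState is a character state for a button-mashing minigame that requires a set number of presses.
; Initialize stores the button and target count, resets the counter and prints an error if the target is not positive.
; A matching primary input plays a sound and increments the counter; reaching the target fires the completion event and switches the owner's state.
; GetProgression exposes the clamped count-to-target ratio.
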(fn IMiniGamePrimaryInput
  (|CallParentFunction)
  (if (Utilities|Enum|Equal(Enum) (Variables|Default|GetbuttonToSpam) "NewEnumerator0")
    (Audio|PlaySound2D (Variables|Default|GetsoundOnInputPress) 1.0 1.0 0.0 0 0)
    (bind _result (Math|Integer|IncrementInt (Variables|Default|GetcurrentCount))
      (:%20%20
        ;[1 1 1] Has been minigame is complete?
        (if (>= _result (Variables|Default|GetcountToSpam))
          (Default|CallOnMinigameComplete)
          (Default|SetState (Variables|Default|GetOwner) "NewEnumerator0"))))))

(fn Initialize
  (params (buttonToSpam :type EMiniGameInput%20Enum :default "NewEnumerator0") (countToSpam :type Integer))
  (Variables|Default|SetbuttonToSpam buttonToSpam)
  (bind _output_get (Variables|Default|SetcountToSpam countToSpam))
  (if (> _output_get 0)
    _
    (else
      (Development|PrintString "ERROR: count to spam is inferior or less than zero")))
  (Variables|Default|SetcurrentCount 0))

(fn GetProgression
  (return (Math|Float|Clamp(Float) (/ (Math|Conversions|ToFloat(Integer) (Variables|Default|GetcurrentCount)) (Math|Conversions|ToFloat(Integer) (Variables|Default|GetcountToSpam))))))