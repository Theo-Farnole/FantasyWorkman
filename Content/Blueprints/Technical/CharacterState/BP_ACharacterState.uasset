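; Base character state that stores its owning character and supplies default handlers for movement, interact and carry input.
; Grab asks the owner's character detection component for the nearest carriable and hands it to the carrier, while ungrab and throw call the carrier directly, with throw first checking that it is allowed.
; Movement and interact handlers are empty here.
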(fn IUpDown
  (params (axisValue :type Float%20%28single-precision%29)))

(fn ILeftRight
  (params (axisValue :type Float%20%28single-precision%29)))

(fn SetOwner
  (params (Owner :type CH%20Third%20Person%20Object%20Reference))
  (Variables|Default|SetOwner Owner))

(fn IStartInteract)

(fn IEndInteract)

(fn IGrabItem
  (bind (_iscarriable _carriable) (Default|GetNearestCarriable (Variables|/Game/Blueprints/Gamemodes/Game/CH_ThirdPerson.CH_ThirdPerson_C|GetBPC_CharacterDetection (Variables|Default|GetOwner))))
  (if _iscarriable
    (Default|Carry (Utilities|GetCarrier) _carriable "0, 0, 0")))

(fn IUngrabItem
  (Default|Uncarry (Utilities|GetCarrier)))

(fn IThrowItem
  (bind _bp_carrier (Utilities|GetCarrier))
  (bind _canthrow (Default|CanThrowCarriedObject _bp_carrier))
  (if _canthrow
    (Default|ThrowCarriedObject _bp_carrier)))