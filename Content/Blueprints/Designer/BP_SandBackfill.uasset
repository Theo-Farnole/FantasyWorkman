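; BP_SandBackfill is an interactable backfill spot that the player fills by bringing buckets of sand.
; Interacting checks the CH_ThirdPerson's carried BP_Bucket for sand, then increments the fill count, refreshes the visual and resets the bucket's content, or prints an error.
; UpdateVisual uses IsFill to pick the unstarted or finished mesh and clear the outline when full.
; Hovering toggles the Outliner highlight only while unfilled.
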(event EventStartInteract
  (params (interactActor :type Actor%20Object%20Reference))
  (bind _asch_third_person (Utilities|Casting|CastToCH_ThirdPerson interactActor))
  (bind _asbp_bucket (Utilities|Casting|CastToBP_Bucket (Variables|/Game/Blueprints/Technical/Components/BPC_Carrier.BPC_Carrier_C|GetcarriedObject (Variables|/Game/Blueprints/Gamemodes/Game/CH_ThirdPerson.CH_ThirdPerson_C|GetBP_Carrier _asch_third_person)))
    (:then
      (if (Utilities|Enum|Equal(Enum) (Variables|/Game/Blueprints/Designer/BP_Bucket.BP_Bucket_C|Getcontent _asbp_bucket) "NewEnumerator1")
        (Math|Integer|IncrementInt (Variables|Default|GetcurrentNumbersOfContent)
          (:%20%20
            (Utilities|UpdateVisual)
            (Default|SetContent _asbp_bucket "NewEnumerator0")))
        (else
          (Development|PrintString "ERROR: Character must carry a bucket of sand to backfill." :!label _label))))
    (:CastFailed
      (goto _label))))

(event EventStopInteract
  (params (interactActor :type Actor%20Object%20Reference)))

(event EventBeginPlay
  (Utilities|UpdateVisual))

(event EventStartHover
  (params (hoverActor :type Actor%20Object%20Reference))
  (if (not (Utilities|IsFill))
    (Default|ShowOutline (Variables|Default|GetOutliner))))

(event EventEndHover
  (params (hoverActor :type Actor%20Object%20Reference))
  (if (not (Utilities|IsFill))
    (Default|HideOutline (Variables|Default|GetOutliner))))

(fn ConstructionScript)