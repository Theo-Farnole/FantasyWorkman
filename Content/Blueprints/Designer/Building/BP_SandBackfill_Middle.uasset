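; Interactable backfill point, the middle sand variant by name, that players fill using buckets of sand.
; CanInteract passes only while it is not full and the third-person character carries a BP_Bucket with the required content.
; On StartInteract it empties that bucket and increments its content count.
; GetSprite supplies the backfill icon, dirt-bucket need indicator and A-button prompt.
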(event EventStartInteract
  (params (interactActor :type Actor%20Object%20Reference))
  (bind _isinteractable (CallFunction|CanInteract interactActor))
  (if _isinteractable
    ;[1 1 1] Get bucket, and empty it.
    (bind _asch_third_person (Utilities|Casting|CastToCH_ThirdPerson interactActor))
    (bind _asbp_bucket (Utilities|Casting|CastToBP_Bucket (Variables|/Game/Blueprints/Technical/Components/BPC_Carrier.BPC_Carrier_C|GetcarriedObject (Variables|/Game/Blueprints/Gamemodes/Game/CH_ThirdPerson.CH_ThirdPerson_C|GetBP_Carrier _asch_third_person))))
    (Default|EmptyBucket _asbp_bucket)
    (CallFunction|IncrementCurrentNumbersOfContent)))

(fn ConstructionScript)

(fn GetSprite
  (return "/Game/Art/UI/Icon/SPR_Icon_Backfill.SPR_Icon_Backfill" "/Game/Art/UI/Circle_RedBar/SPR_Circle_RedBar_Bucket_Dirt.SPR_Circle_RedBar_Bucket_Dirt" "/Game/Art/UI/Button/SPR_Button_A.SPR_Button_A"))

(fn CanInteract
  (params (interactActor :type Actor%20Object%20Reference))
  (bind _isfill (CallFunction|IsFill))
  (if _isfill
    _
    (else
      (bind _asch_third_person (Utilities|Casting|CastToCH_ThirdPerson interactActor)
        (:then
          (bind _asbp_bucket (Utilities|Casting|CastToBP_Bucket (Variables|/Game/Blueprints/Technical/Components/BPC_Carrier.BPC_Carrier_C|GetcarriedObject (Variables|/Game/Blueprints/Gamemodes/Game/CH_ThirdPerson.CH_ThirdPerson_C|GetBP_Carrier _asch_third_person)))
            (:then
              (if (Utilities|Enum|Equal(Enum) (Variables|/Game/Blueprints/Designer/Items/BP_Bucket.BP_Bucket_C|Getcontent _asbp_bucket) "NewEnumerator1")
                (return true)
                (else
                  (Development|PrintString "ERROR: Character must carry a bucket of sand to backfill."))))
            (:CastFailed
              _)))
        (:CastFailed
          _))))
  (return false))