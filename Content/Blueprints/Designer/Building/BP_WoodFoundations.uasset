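; BP_WoodFoundations is a building-stage interactable that players fill with carried wood planks to construct wood foundations.
; CanInteract passes only when a CH_ThirdPerson carries a BP_WoodPlank, printing an error if that character carries anything else or nothing.
; StartInteract calls the parent, then on a valid check destroys the carried item and increments the inherited content count.
; GetSprite supplies the scaffolding, required-plank and input-button icons.
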(event EventStartInteract
  (params (interactActor :type Actor%20Object%20Reference))
  (|CallParentFunction interactActor)
  (bind _isinteractable (CallFunction|CanInteract interactActor))
  (if _isinteractable
    (bind _asch_third_person (Utilities|Casting|CastToCH_ThirdPerson interactActor))
    (Default|DestroyCarryItem (Variables|/Game/Blueprints/Gamemodes/Game/CH_ThirdPerson.CH_ThirdPerson_C|GetBP_Carrier _asch_third_person))
    (CallFunction|IncrementCurrentNumbersOfContent)))

(fn ConstructionScript
  (|CallParentFunction))

(fn GetSprite
  (return "/Game/Art/UI/Icon/SPR_Icon_Scaffolding.SPR_Icon_Scaffolding" "/Game/Art/UI/Circle_RedBar/SPR_Circle_RedBar_Wood_Plank.SPR_Circle_RedBar_Wood_Plank" "/Game/Art/UI/Button/SPR_Button_A.SPR_Button_A"))

(fn CanInteract
  (params (interactActor :type Actor%20Object%20Reference))
  (bind _asch_third_person (Utilities|Casting|CastToCH_ThirdPerson interactActor)
    (:then
      (Utilities|Casting|CastToBP_WoodPlank (Utilities|ToObject(Interface) (Variables|/Game/Blueprints/Technical/Components/BPC_Carrier.BPC_Carrier_C|GetcarriedObject (Variables|/Game/Blueprints/Gamemodes/Game/CH_ThirdPerson.CH_ThirdPerson_C|GetBP_Carrier _asch_third_person)))
        (:then
          (return true))
        (:CastFailed
          (Development|PrintString "ERROR: To build wood foundations, you must carry wood plank."))))
    (:CastFailed
      _))
  (return false))