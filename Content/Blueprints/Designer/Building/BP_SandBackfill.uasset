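; BP_SandBackfill is an interactable backfill spot that the player fills with buckets of sand.
; On StartInteract, if not already full, it casts the interactor to CH_ThirdPerson and checks its carrier for a BP_Bucket with the required content.
; A valid bucket increments the fill count and has its content reset; otherwise an error is printed saying a bucket of sand is required.
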(event EventStartInteract
  (params (interactActor :type Actor%20Object%20Reference))
  (bind _isfill (CallFunction|IsFill))
  (if (not _isfill)
    (bind _asch_third_person (Utilities|Casting|CastToCH_ThirdPerson interactActor))
    (bind _asbp_bucket (Utilities|Casting|CastToBP_Bucket (Variables|/Game/Blueprints/Technical/Components/BPC_Carrier.BPC_Carrier_C|GetcarriedObject (Variables|/Game/Blueprints/Gamemodes/Game/CH_ThirdPerson.CH_ThirdPerson_C|GetBP_Carrier _asch_third_person)))
      (:then
        (if (Utilities|Enum|Equal(Enum) (Variables|/Game/Blueprints/Designer/Items/BP_Bucket.BP_Bucket_C|Getcontent _asbp_bucket) "NewEnumerator1")
          (CallFunction|IncrementCurrentNumbersOfContent)
          (Default|SetContent _asbp_bucket "NewEnumerator0")
          (else
            (Development|PrintString "ERROR: Character must carry a bucket of sand to backfill." :!label _label))))
      (:CastFailed
        (goto _label)))))

(fn ConstructionScript)