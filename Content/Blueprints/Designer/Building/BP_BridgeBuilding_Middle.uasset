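; BP_BridgeBuilding_Middle is the middle bridge building piece, which characters fill by delivering carried rocks.
; On StartInteract, if not yet full, it checks the character's BPCarrier for a BP_Rock, uncarries and destroys it, then increments its content count; any other cargo prints an error.
; GetSprite supplies the bridge rock icon, rock progress indicator and A-button prompt.
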(event EventBeginPlay
  (|CallParentFunction) ; This node is disabled and will not be called.\nDrag off pins to build functionality.
)

(event EventStartInteract
  (params (interactActor :type Actor%20Object%20Reference))
  (bind _isfill (CallFunction|IsFill))
  (if (not _isfill)
    (bind _asch_third_person (Utilities|Casting|CastToCH_ThirdPerson interactActor))
    (bind _asbp_rock (Utilities|Casting|CastToBP_Rock (Utilities|ToObject(Interface) (Variables|/Game/Blueprints/Technical/Components/BPC_Carrier.BPC_Carrier_C|GetcarriedObject (Variables|/Game/Blueprints/Gamemodes/Game/CH_ThirdPerson.CH_ThirdPerson_C|GetBP_Carrier _asch_third_person))))
      (:then
        (Default|Uncarry (Variables|/Game/Blueprints/Gamemodes/Game/CH_ThirdPerson.CH_ThirdPerson_C|GetBP_Carrier _asch_third_person) true)
        (Actor|DestroyActor _asbp_rock)
        (CallFunction|IncrementCurrentNumbersOfContent))
      (:CastFailed
        (Development|PrintString "ERROR: Character must carry rock.")))))

(fn ConstructionScript
  (|CallParentFunction))

(fn GetSprite
  (return "/Game/Art/UI/Icon/SPR_Icon_Bridge_Rocks.SPR_Icon_Bridge_Rocks" "/Game/Art/UI/Circle_RedBar/SPR_Circle_RedBar_Rock.SPR_Circle_RedBar_Rock" "/Game/Art/UI/Button/SPR_Button_A.SPR_Button_A"))