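; BP_BridgeBuilding is a bridge construction site that the player builds up by delivering carried rocks.
; On interact, if it is not yet full, it checks the third-person character's carrier component for a BP_Rock.
; A carried rock is released, destroyed and added to the content count; anything else prints an error.
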(event EventBeginPlay
  (|CallParentFunction) ; This node is disabled and will not be called.\nDrag off pins to build functionality.
)

(event EventStartInteract
  (params (interactActor :type Actor%20Object%20Reference))
  (bind _isfill (CallFunction|IsFill))
  (if (not _isfill)
    (bind _asch_third_person (Utilities|Casting|CastToCH_ThirdPerson interactActor))
    (bind _asbp_rock (Utilities|Casting|CastToBP_Rock (Utilities|ToObject(Interface) (Variables|/Game/Blueprints/Technical/Components/BPC_Carrier.BPC_Carrier_C|GetcarriedObject (Variables|/Game/Blueprints/Gamemodes/Game/CH_ThirdPerson.CH_ThirdPerson_C|GetBP_Carrier _asch_third_person))))
      (:then
        (Default|Uncarry (Variables|/Game/Blueprints/Gamemodes/Game/CH_ThirdPerson.CH_ThirdPerson_C|GetBP_Carrier _asch_third_person))
        (Actor|DestroyActor _asbp_rock)
        (CallFunction|IncrementCurrentNumbersOfContent))
      (:CastFailed
        (Development|PrintString "ERROR: Character must carry rock.")))))

(fn ConstructionScript
  (|CallParentFunction))