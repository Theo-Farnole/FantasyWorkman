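; BP_Bucket is a carryable bucket that holds one content type: empty, sand, water or concrete.
; It can always be carried but can be thrown only when empty, and exposes its static mesh as the carriable component.
; Setting or emptying the content refreshes a separate content mesh from a material map, hiding it for a null material and printing an error for a missing entry.
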(event EventBeginPlay
  (Utilities|UpdateContentVisual))

(fn ConstructionScript)

(fn EmptyBucket
  (CallFunction|SetContent "NewEnumerator0"))

(fn SetContent
  (params (newContent :type EBucketContent%20Enum :default "NewEnumerator0"))
  (Variables|Default|Setcontent newContent)
  (Utilities|UpdateContentVisual))

(fn CanCarry
  (params (Carrier :type BPC%20Carrier%20Object%20Reference))
  (return true))

(fn CanThrow
  (switch Utilities|FlowControl|Switch|SwitchonEBucketContent (Variables|Default|Getcontent)
    (:NewEnumerator0
      (return true))
    (:NewEnumerator1
      _)
    (:NewEnumerator2
      _)
    (:NewEnumerator3
      _))
  (return false))

(fn GetCariableComponent
  (return (Variables|Default|GetStaticMesh)))