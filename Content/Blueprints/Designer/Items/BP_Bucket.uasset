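; Bucket item that holds one content type (empty, sand, water or concrete) and can be thrown only while empty.
; SetContent stores the new type and refreshes the visual, which is also updated on BeginPlay; emptying and resetting both route through it.
; The visual looks up a material per content, hides the content mesh when that material is invalid, and prints an error when none is found.
; It also supplies its UI icon sprites.
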(event EventBeginPlay
  (Utilities|UpdateContentVisual))

(event EventOnReset
  (CallFunction|SetContent "NewEnumerator0"))

(fn ConstructionScript)

(fn EmptyBucket
  (CallFunction|SetContent "NewEnumerator0"))

(fn SetContent
  (params (newContent :type EBucketContent%20Enum :default "NewEnumerator0"))
  (Variables|Default|Setcontent newContent)
  (Utilities|UpdateContentVisual))

(fn GetSprite
  (return "/Game/Art/UI/Icon/SPR_Icon_Bucket.SPR_Icon_Bucket" "/Game/Art/UI/Circle_RedBar/SPR_Circle_RedBar_Bucket.SPR_Circle_RedBar_Bucket" "/Game/Art/UI/Button/SPR_Button_A.SPR_Button_A"))

(fn CanThrow
  (switch Utilities|FlowControl|Switch|SwitchonEBucketContent (Variables|Default|Getcontent)
    (:NewEnumerator0
      (return true))
    (:NewEnumerator1
      _)
    (:NewEnumerator2
      _)
    (:NewEnumerator3
      _))
  (return false))