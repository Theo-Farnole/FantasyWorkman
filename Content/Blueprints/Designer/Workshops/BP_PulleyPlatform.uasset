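; Pulley platform that moves between Start and End points and carries up to four carriable actors.
; Each overlap box claims an entering BP_ICarriable for its empty slot, disabling its gravity and switching collision to IgnoreOnlyPawn.
; Tick pins occupants to slot transforms, and leaving the box restores gravity and clears the slot.
; GoToEnd and GoToStart lerp the platform by a passed-in alpha and set IsOnFloor.
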(event OnComponentBeginOverlap(Box1)
  (params (OverlappedComponent :type Primitive%20Component%20Object%20Reference) (OtherActor :type Actor%20Object%20Reference) (OtherComp :type Primitive%20Component%20Object%20Reference) (OtherBodyIndex :type Integer) (bFromSweep :type Boolean) (SweepResult :type Hit%20Result%20Structure%20%28by%20ref%29))
  ;[1 1 1] Slot2
  (Utilities|GetSnaptoPlatform OtherActor (Variables|Default|GetActorCarrySlot2)))

(event OnComponentBeginOverlap(Box)
  (params (OverlappedComponent :type Primitive%20Component%20Object%20Reference) (OtherActor :type Actor%20Object%20Reference) (OtherComp :type Primitive%20Component%20Object%20Reference) (OtherBodyIndex :type Integer) (bFromSweep :type Boolean) (SweepResult :type Hit%20Result%20Structure%20%28by%20ref%29))
  ;[1 1 1] Slot 1
  (Utilities|GetSnaptoPlatform OtherActor (Variables|Default|GetactorCarrySlot1)))

(event OnComponentEndOverlap(Box)
  (params (OverlappedComponent :type Primitive%20Component%20Object%20Reference) (OtherActor :type Actor%20Object%20Reference) (OtherComp :type Primitive%20Component%20Object%20Reference) (OtherBodyIndex :type Integer))
  ;[1 1 1] Slot 1
  (Utilities|OnUnSnapPlatform OtherActor (Variables|Default|GetactorCarrySlot1)))

(event OnComponentEndOverlap(Box1)
  (params (OverlappedComponent :type Primitive%20Component%20Object%20Reference) (OtherActor :type Actor%20Object%20Reference) (OtherComp :type Primitive%20Component%20Object%20Reference) (OtherBodyIndex :type Integer))
  ;[1 1 1] Slot2
  (Utilities|OnUnSnapPlatform OtherActor (Variables|Default|GetActorCarrySlot2)))

(event OnComponentBeginOverlap(Box2)
  (params (OverlappedComponent :type Primitive%20Component%20Object%20Reference) (OtherActor :type Actor%20Object%20Reference) (OtherComp :type Primitive%20Component%20Object%20Reference) (OtherBodyIndex :type Integer) (bFromSweep :type Boolean) (SweepResult :type Hit%20Result%20Structure%20%28by%20ref%29))
  ;[1 1 1] Slot 3
  (Utilities|GetSnaptoPlatform OtherActor (Variables|Default|GetActorCarrySlot3)))

(event OnComponentEndOverlap(Box2)
  (params (OverlappedComponent :type Primitive%20Component%20Object%20Reference) (OtherActor :type Actor%20Object%20Reference) (OtherComp :type Primitive%20Component%20Object%20Reference) (OtherBodyIndex :type Integer))
  ;[1 1 1] Slot 3
  (Utilities|OnUnSnapPlatform OtherActor (Variables|Default|GetActorCarrySlot3)))

(event OnComponentBeginOverlap(Box3)
  (params (OverlappedComponent :type Primitive%20Component%20Object%20Reference) (OtherActor :type Actor%20Object%20Reference) (OtherComp :type Primitive%20Component%20Object%20Reference) (OtherBodyIndex :type Integer) (bFromSweep :type Boolean) (SweepResult :type Hit%20Result%20Structure%20%28by%20ref%29))
  ;[1 1 1] Slot 4
  (Utilities|GetSnaptoPlatform OtherActor (Variables|Default|GetActorCarrySlot4)))

(event OnComponentEndOverlap(Box3)
  (params (OverlappedComponent :type Primitive%20Component%20Object%20Reference) (OtherActor :type Actor%20Object%20Reference) (OtherComp :type Primitive%20Component%20Object%20Reference) (OtherBodyIndex :type Integer))
  ;[1 1 1] Slot 4
  (Utilities|OnUnSnapPlatform OtherActor (Variables|Default|GetActorCarrySlot4)))

(event EventBeginPlay)

(event EventTick
  (params (DeltaSeconds :type Float%20%28single-precision%29))
  (Utilities|SetTransformonPlatform))

(fn ConstructionScript)

(fn GotoEnd
  (params (value :type Float%20%28single-precision%29))
  (Transformation|SetActorLocation (Math|Vector|Lerp(Vector) (Variables|Default|Getstart) (Variables|Default|Getend) value) false false)
  (Variables|Default|SetisOnFloor true))

(fn GotoStart
  (params (value :type Float%20%28single-precision%29))
  (Transformation|SetActorLocation (Math|Vector|Lerp(Vector) (Variables|Default|Getend) (Variables|Default|Getstart) value) false false)
  (Variables|Default|SetisOnFloor false))

(fn SetVariable
  (params (Slot :type Actor%20Object%20Reference%20%28by%20ref%29) (ActorRef :type Actor%20Object%20Reference))
  (|SetBy-RefVar Slot ActorRef)
  (return))

(fn SetTransformonSlot
  (params (ActorSet :type Actor%20Object%20Reference) (Slot :type Scene%20Component%20Object%20Reference))
  (Transformation|SetActorRelativeTransform ActorSet (Math|Transform|MakeTransform (Transformation|GetWorldLocation Slot) (Transformation|GetWorldRotation Slot)) false false)
  (bind _asbp_icarriable (Utilities|Casting|CastToBP_ICarriable ActorSet))
  (bind _cariablecomponent (Default|GetCariableComponent _asbp_icarriable))
  (Physics|SetEnableGravity _cariablecomponent false))