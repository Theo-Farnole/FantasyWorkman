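; BP_ChopChop is a workshop that turns a carried wood log into crafted items through a button-spam minigame.
; Interaction is refused if occupied or without a log; otherwise it consumes the log and puts the character into BP_SpamInputState.
; Minigame completion spawns ToSpawn using actor-relative SpawnPositions and clears the interactor, which also feeds the progress bar widget.
; The construction script draws debug spheres at spawn positions.
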(event Custom|OnMinigameComplete
  (Utilities|SpawnCraftedItems)
  (CallFunction|SetInteractor))

(event EventBeginPlay
  (|CallParentFunction)
  (Utilities|IstoSpawnClassValid))

(event EventStartInteract
  (params (interactActor :type Actor%20Object%20Reference))
  (Utilities|IsValid (Variables|Default|Getinteractor)
    (:Is%20Valid
      (Development|PrintString "ERROR: cannot use the Chop Chop workshop:another character is using it."))
    (:Is%20Not%20Valid
      (bind _asch_third_person (Utilities|Casting|CastToCH_ThirdPerson interactActor))
      (Utilities|Casting|CastToBP_WoodLog (Variables|/Game/Blueprints/Technical/Components/BPC_Carrier.BPC_Carrier_C|GetcarriedObject (Variables|/Game/Blueprints/Gamemodes/Game/CH_ThirdPerson.CH_ThirdPerson_C|GetBP_Carrier _asch_third_person))
        (:then
          (bind _asbp_spam_input_state (Utilities|StartCraft _asch_third_person))
          (EventDispatchers|AssignOnMinigameComplete _asbp_spam_input_state (delegate Custom|OnMinigameComplete)))
        (:CastFailed
          (Development|PrintString "ERROR: Character must carry a wood log to use the Chop Chop workshop."))))))

(fn ConstructionScript
  (|CallParentFunction)
  (Rendering|Debug|FlushPersistentDebugLines)
  (Utilities|DebugDrawSpawnPositions))

(fn GetSprite
  (return "/Game/Art/UI/Icon/SPR_Icon_Wood_Log.SPR_Icon_Wood_Log" "/Game/Art/UI/Button/SPR_Button_A.SPR_Button_A" "/Game/Art/UI/Circle_RedBar/SPR_Circle_RedBar_Wood_Log.SPR_Circle_RedBar_Wood_Log"))

(fn SetInteractor
  (params (interactor :type CH%20Third%20Person%20Object%20Reference))
  (Utilities|IsValid interactor
    (:Is%20Valid
      (Default|HideWidget (Variables|/Game/Blueprints/Gamemodes/Game/CH_ThirdPerson.CH_ThirdPerson_C|GetBPC_UIWidgeUpdate interactor)))
    (:Is%20Not%20Valid
      _))
  (bind _output_get (Variables|Default|Setinteractor interactor))
  (bind _aswbp_workshop_progress_bar (Utilities|Casting|CastToWBP_WorkshopProgressBar (UserInterface|GetUserWidgetObject (Variables|Default|GetProgressBar))))
  (Variables|/Game/Blueprints/Widgets/WBP_WorkshopProgressBar.WBP_WorkshopProgressBar_C|Setinteractor _aswbp_workshop_progress_bar _output_get))