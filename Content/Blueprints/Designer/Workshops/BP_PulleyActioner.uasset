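; BP_PulleyActioner is an interactable that moves a linked Platform between its start and end positions.
; On interaction, a direction check ignores the input while the platform is busy, otherwise locks it and branches on whether it is on the floor.
; Separate timelines drive the platform's GoToStart or GoToEnd each update and unlock it when finished.
; GetSprite supplies a wooden log sprite.
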(event EventBeginPlay
  (|CallParentFunction) ; This node is disabled and will not be called.\nDrag off pins to build functionality.
)

(event EventStartInteract
  (params (interactActor :type Actor%20Object%20Reference))
  (Utilities|WhichDirection
    (:then
      (bind _test (Timeline|Timeline_0 PlayFromStart)
        (:Update
          (Utilities|GotoStart _test :!label _label))
        (:Finished
          (goto _label finish))))
    (:else
      (bind _test_2 (Timeline|Timeline PlayFromStart)
        (:Update
          (Utilities|GotoEnd _test_2 :!label _label_2))
        (:Finished
          (goto _label_2 finish))))))

(fn ConstructionScript
  (|CallParentFunction))

(fn GetSprite
  (return "/Game/Art/UI/Circle/SPR_Circle_Wood_Log_Sprite.SPR_Circle_Wood_Log_Sprite" 0))