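; Piston-style pulley actioner that, on interaction, drives a linked Platform between its start and end positions.
; A direction macro ignores input while the platform is busy, locks it, then picks the travel direction from whether it is on the floor.
; Timelines feed the platform's movement and spin the crank in opposite directions per trip, releasing the lock when finished.
; It also supplies piston and joystick sprites for icons.
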(event EventBeginPlay
  (|CallParentFunction) ; This node is disabled and will not be called.\nDrag off pins to build functionality.
)

(event EventStartInteract
  (params (interactActor :type Actor%20Object%20Reference))
  (Utilities|WhichDirection
    (:then
      (bind _test (Timeline|Timeline_0 PlayFromStart)
        (:Update
          (Utilities|GotoStart _test :!label _label))
        (:Finished
          (goto _label finish))))
    (:else
      (bind _test_2 (Timeline|Timeline PlayFromStart)
        (:Update
          (Utilities|GotoEnd _test_2 :!label _label_2))
        (:Finished
          (goto _label_2 finish))))))

(fn ConstructionScript
  (|CallParentFunction))

(fn GetSprite
  (return "/Game/Art/UI/Icon/SPR_Icon_Piston.SPR_Icon_Piston" 0 "/Game/Art/UI/Button/SPR_Button_Joystick.SPR_Button_Joystick"))