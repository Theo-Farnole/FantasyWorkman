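; Game mode for a timed match that runs the countdown, handles winning and losing, and rates the result in stars.
; BeginPlay creates an extra local player, adds the main HUD widget, starts music and hides the cursor.
; Tick accumulates elapsed time, updates the HUD countdown and calls Lose at the time limit.
; Win and Lose show the end screen with time-based stars and duration, restore the cursor and stop the game-running flag.
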(event EventTick
  (params (DeltaSeconds :type Float%20%28single-precision%29))
  (Variables|Default|SetcurrentGameDuration (+ DeltaSeconds (Variables|Default|GetcurrentGameDuration)))
  (Utilities|UpdateWidgetTimer)
  (Utilities|ManageLosefromTimer))

(event EventBeginPlay
  (Class|GameplayStatics|CreatePlayer -1)
  (bind _returnvalue (UserInterface|CreateWidget "/Game/Blueprints/Widgets/WPB_DimiTechnicalShowcase.WPB_DimiTechnicalShowcase_C"))
  (bind _output_get (Variables|Default|SetmainWidget _returnvalue))
  (UserInterface|Viewport|AddtoPlayerScreen _output_get -1)
  (Audio|PlaySound2D "/Game/Sounds/S_GameMusic.S_GameMusic" 1.0 1.0 0.0 0 0)
  (Variables|/Script/Engine.PlayerController|SetbShowMouseCursor (Game|GetPlayerController 0) false))

(fn ConstructionScript)

(fn Win
  (Development|PrintString "GM_Game: Win")
  (bind _returnvalue (UserInterface|CreateWidget "/Game/Blueprints/Widgets/WBP_EndGame.WBP_EndGame_C"))
  (UserInterface|Viewport|AddtoViewport _returnvalue 0)
  (Default|Initialize _returnvalue true (Utilities|GetStarsCount) (Variables|Default|GetcurrentGameDuration))
  (Variables|/Script/Engine.PlayerController|SetbShowMouseCursor (Game|GetPlayerController 0) true)
  (Variables|Default|SetisGameRunning false))

(fn Lose
  (Development|PrintString "GM_Game: Lose")
  (bind _returnvalue (UserInterface|CreateWidget "/Game/Blueprints/Widgets/WBP_EndGame.WBP_EndGame_C"))
  (UserInterface|Viewport|AddtoViewport _returnvalue 0)
  (Default|Initialize _returnvalue false (Utilities|GetStarsCount) (Variables|Default|GetmaxGameDuration))
  (Variables|/Script/Engine.PlayerController|SetbShowMouseCursor (Game|GetPlayerController 0) true)
  (Variables|Default|SetisGameRunning false))