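; PC_Game is a player controller Blueprint that provides debug hotkeys for construction and game speed.
; Tab flips a dependency-requirement flag and copies it to every existing BP_AConstructionToBuild actor, printing the new state.
; Numpad 1 toggles instant build through BP_CheatManager.
; The Add and Subtract keys step global time dilation up or down and print the result.
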(event Input|KeyboardEvents|Tab
  (params (Key :type Key%20Structure :default "None"))
  (:Pressed
    (CallFunction|ToggleDependenciesRequirement)))

(event Input|KeyboardEvents|Subtract
  (params (Key :type Key%20Structure :default "None"))
  (:Pressed
    (Utilities|Time|SetGlobalTimeDilation (- (Class|GameplayStatics|GetGlobalTimeDilation) (Variables|Default|GettimeDilatationStep)))
    (Utilities|PrintDilationChangement)))

(event Input|KeyboardEvents|NumPadOne
  (params (Key :type Key%20Structure :default "None"))
  (:Pressed
    (bind _asbp_cheat_manager (Utilities|Casting|CastToBP_CheatManager (Variables|Default|GetCheatManager)))
    (Default|ToggleInstantBuild _asbp_cheat_manager)))

(event Input|KeyboardEvents|Add
  (params (Key :type Key%20Structure :default "None"))
  (:Pressed
    (Utilities|Time|SetGlobalTimeDilation (+ (Class|GameplayStatics|GetGlobalTimeDilation) (Variables|Default|GettimeDilatationStep)))
    (Utilities|PrintDilationChangement)))

(fn ConstructionScript)

(fn ToggleDependenciesRequirement
  (bind _output_get (Variables|Default|SetdependenciesEnabled (not (Variables|Default|GetdependenciesEnabled))))
  (if _output_get
    (Development|PrintString "ENABLE DEPENDENCIES")
    (else
      (Development|PrintString "DISABLE  DEPENDENCIES")))
  (bind _outactors (Actor|GetAllActorsOfClass "/Game/Blueprints/Technical/BaseClasses/BP_AConstructionToBuild.BP_AConstructionToBuild_C"))
  (for _array_element _outactors
    (Variables|/Game/Blueprints/Technical/BaseClasses/BP_AConstructionToBuild.BP_AConstructionToBuild_C|SetenableDependencies _array_element (Variables|Default|GetdependenciesEnabled))))