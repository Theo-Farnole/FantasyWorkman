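; BP_SplineDecalPlacer is a construction-script tool that lays decals along a spline, such as over ground surfaces.
; It first snaps each spline point to geometry with a vertical Visibility trace within a threshold.
; It then adds decal components at intervals derived from decal scale and offset, with a capped count.
; Each decal projects vertically, follows the spline's yaw and roll, and alternates between two materials.
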(event EventBeginPlay)

(event Collision|EventActorBeginOverlap
  (params (OtherActor :type Actor%20Object%20Reference)))

(event EventTick
  (params (DeltaSeconds :type Float%20%28single-precision%29)))

(fn ConstructionScript
  (bind _decalscale (Variables|Default|GetDecalScale))
  (Utilities|FlowControl|Sequence
    (:then_0
      ;[1 1 1] Snap Spline Point To Surface
      (for _index (range 0 (- (Spline|GetNumberOfSplinePoints (Variables|Default|GetSplineDecalPlacer)) 1))
        (bind (_outhit _returnvalue) (Collision|LineTraceByChannel (Math|Vector|MakeVector (.x (Spline|GetLocationatSplinePoint (Variables|Default|GetSplineDecalPlacer) _index "World")) (.y (Spline|GetLocationatSplinePoint (Variables|Default|GetSplineDecalPlacer) _index "World")) (+ (.z (Spline|GetLocationatSplinePoint (Variables|Default|GetSplineDecalPlacer) _index "World")) (Variables|Default|GetDecalSnapThreshold))) (Math|Vector|MakeVector (.x (Spline|GetLocationatSplinePoint (Variables|Default|GetSplineDecalPlacer) _index "World")) (.y (Spline|GetLocationatSplinePoint (Variables|Default|GetSplineDecalPlacer) _index "World")) (- (.z (Spline|GetLocationatSplinePoint (Variables|Default|GetSplineDecalPlacer) _index "World")) (Variables|Default|GetDecalSnapThreshold))) "TraceTypeQuery1" false 0 "None" true "(R=1.000000,G=0.000000,B=0.000000,A=1.000000)" "(R=0.000000,G=1.000000,B=0.000000,A=1.000000)" 2.0))
        (if _returnvalue
          (Spline|SetLocationatSplinePoint (Variables|Default|GetSplineDecalPlacer) _index (.location _outhit) "World" true))))
    (:then_1
      (for _index_2 (range 0 (Math|Float|Truncate (Math|Float|Clamp(Float) (/ (Spline|GetSplineLength (Variables|Default|GetSplineDecalPlacer)) (* (* (Variables|Default|GetDecalScale) 512.0) (Variables|Default|GetDecalOffset))) 0.0 1e+02)))
        (bind _returnvalue_2 (AddComponent|AddDecalComponent false (Math|Transform|MakeTransform "0, 0, 0" "90.000000, 0, 0" (Math|Vector|MakeVector (Variables|Default|GetProjectionScale) _decalscale _decalscale))))
        (Transformation|SetWorldLocationAndRotation _returnvalue_2 (Spline|GetLocationatDistanceAlongSpline (Variables|Default|GetSplineDecalPlacer) (* _index_2 (* (* (Variables|Default|GetDecalScale) 512.0) (Variables|Default|GetDecalOffset))) "World") (Math|Rotator|MakeRotator (.roll (Spline|GetRotationatDistanceAlongSpline (Variables|Default|GetSplineDecalPlacer) (* _index_2 (* (* (Variables|Default|GetDecalScale) 512.0) (Variables|Default|GetDecalOffset))) "World")) 9e+01 (.yaw (Spline|GetRotationatDistanceAlongSpline (Variables|Default|GetSplineDecalPlacer) (* _index_2 (* (* (Variables|Default|GetDecalScale) 512.0) (Variables|Default|GetDecalOffset))) "World"))) false false)
        (if (== (Math|Integer|%(Integer) _index_2 2) 0)
          (Rendering|Components|Decal|SetDecalMaterial _returnvalue_2 (Utilities|Array|Get(acopy) (Variables|Default|GetDecalToPlace)))
          (else
            (Rendering|Components|Decal|SetDecalMaterial _returnvalue_2 (Utilities|Array|Get(acopy) (Variables|Default|GetDecalToPlace) 1))))))))